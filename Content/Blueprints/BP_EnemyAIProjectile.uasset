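; Ranged enemy AI that crouches on spawn, fires projectiles at pawns it sees, and is destroyed when damage depletes its health.
; PawnSensing triggers BP_Projectile spawns, gated by a FireRate delay.
; After each delay, ShouldTurn compares the target's side on the X axis with the enemy's facing, and a Timeline lerps yaw to flip it around if they differ.
; Tick keeps its widget facing the player camera.
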(event `self.ReceiveBeginPlay`
  (`self.Crouch`))

(event `self.PawnSensing.OnSeePawn`
  (params (Pawn :type "Pawn Object Reference"))
  (bind _returnvalue_x (`KismetMathLibrary.BreakVector` (`self.GetActorForwardVector`)))
  ;[1 1 1] Spotting player
  (if (`self.bCanFire`)
    (`|SpawnActorFromClass` "/Game/Blueprints/BP_Projectile.BP_Projectile_C" (`SceneComponent.K2_GetComponentToWorld` (`self.ProjectileSpawnPoint`)) "Undefined" "MultiplyWithRoot" null null)
    (set `self.bCanFire` false)
    (`KismetSystemLibrary.Delay` (`self.FireRate`))
    (set `self.bCanFire` true)
    (bind _newparam (`self.ShouldTurn` Pawn))
    (if _newparam
      (if (> _returnvalue_x 0.0)
        (set `self.RotationToSet` -180.0)
        (bind (_direction _newtrack_0) (`Timeline|Timeline` :!via `PlayFromStart` :!label _label)
          (:`Update`
            (`self.K2_SetActorRotation` (`KismetMathLibrary.RLerp` (`self.K2_GetActorRotation`) (`KismetMathLibrary.MakeRotator` 0.0 0.0 (`self.RotationToSet`)) _newtrack_0))))
        (else
          (set `self.RotationToSet` 0.0)
          (goto _label :!via `PlayFromStart`))))))

(event `self.ReceiveTick`
  (params (DeltaSeconds :type "Float (single-precision)"))
  ;[1 1 1] handle widget camera
  (`|ExecutionSequence`
    (:`then_0`
      (if true
        _))
    (:`then_1`
      (`SceneComponent.K2_SetWorldRotation` (`self.Widget`) (`KismetMathLibrary.FindLookAtRotation` (`SceneComponent.K2_GetComponentLocation` (`self.Widget`)) (`SceneComponent.K2_GetComponentLocation` (`PlayerCameraManager.TransformComponent` (`GameplayStatics.GetPlayerCameraManager` 0)))) false false))))

(event `self.ReceiveAnyDamage`
  (params (Damage :type "Float (single-precision)") (DamageType :type "DamageType Object Reference") (InstigatedBy :type "Controller Object Reference") (DamageCauser :type "Actor Object Reference"))
  ;[1 1 1] handle damage
  (bind _output_get (set `self.Health` (- (`self.Health`) Damage)))
  (`KismetSystemLibrary.PrintString` (`KismetStringLibrary.Conv_DoubleToString` _output_get))
  (if (<= (`self.Health`) 0.0)
    (`self.K2_DestroyActor`)))

(fn `NewFunction`
  (`KismetSystemLibrary.PrintString` "Executeing!"))

(fn `ShouldTurn`
  (params (Player :type "Actor Object Reference"))
  (returns (NewParam :type Boolean))
  (bind _returnvalue_x (`KismetMathLibrary.BreakVector` (`self.K2_GetActorLocation`)))
  (bind _returnvalue_x_2 (`KismetMathLibrary.BreakVector` (`self.K2_GetActorLocation` Player)))
  (bind _returnvalue_x_3 (`KismetMathLibrary.BreakVector` (`self.GetActorForwardVector`)))
  (bind _returnvalue (- _returnvalue_x_2 _returnvalue_x))
  (bind _returnvalue_2 (!= (>= _returnvalue 0.0) (>= _returnvalue_x_3 0.0)))
  (`KismetSystemLibrary.PrintString` (`KismetStringLibrary.Conv_DoubleToString` _returnvalue_x_3))
  (`KismetSystemLibrary.PrintString` (`KismetStringLibrary.Conv_DoubleToString` _returnvalue))
  (`KismetSystemLibrary.PrintString` (`KismetStringLibrary.Conv_BoolToString` _returnvalue_2))
  (return _returnvalue_2))

(fn `UserConstructionScript`)