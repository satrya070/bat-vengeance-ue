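; BaseEnemyTwo is an AI enemy character that patrols, melee-attacks the player and is destroyed at zero health.
; AttackPlayer plays a palm-strike montage, then sphere-traces for pawns to damage the player, gated by a CanAttack cooldown.
; Taking damage sets the player on the Blackboard and ends patrolling.
; Patrol walks to the first waypoint; Patrol2 checks X-axis sight distance; leftover detection logic is disconnected.
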(event `self.ReceiveBeginPlay`)

(event `self.ReceiveTick`
  (params (DeltaSeconds :type "Float (single-precision)")))

(event `AttackPlayer`
  (bind _returnvalue (`self.K2_GetActorLocation`))
  ;[1 1 1] Attacking
  (if (`self.bCanAttack`)
    (set `self.bCanAttack` false)
    (`self.PlayAnimMontage` "/Game/Animations/Paired_CounterPunch_PalmStrike_Att_UE5_Montage.Paired_CounterPunch_PalmStrike_Att_UE5_Montage")
    (`KismetSystemLibrary.Delay` 0.4)
    (bind (_outhit _returnvalue_2) (`KismetSystemLibrary.SphereTraceSingleForObjects` _returnvalue (+ _returnvalue (* (`self.GetActorForwardVector`) (120.0 0.0 0.0))) 0.0 (`|MakeArray` "ObjectTypeQuery3" :!type "EObjectTypeQuery Enum")))
    (if _returnvalue_2
      (bind (_bblockinghit _binitialoverlap _time _distance _location _impactpoint _normal _impactnormal _physmat _hitactor) (`GameplayStatics.BreakHitResult` _outhit))
      (cast `/Game/ThirdPerson/Blueprints/BP_ThirdPersonCharacter` _hitactor)
      (`GameplayStatics.ApplyDamage` _hitactor 5.0)
      (`KismetSystemLibrary.DrawDebugSphere` (`self.K2_GetActorLocation` _hitactor) 120.0 12 (struct :`R` 1.0 :`G` 1.0 :`B` 1.0 :`A` 1.0) 3.0))
    (`KismetSystemLibrary.Delay` 0.7)
    (set `self.bCanAttack` true)))

(event `self.ReceiveAnyDamage`
  (params (Damage :type "Float (single-precision)") (DamageType :type "DamageType Object Reference") (InstigatedBy :type "Controller Object Reference") (DamageCauser :type "Actor Object Reference"))
  ;[1 1 1] Handle Damage
  (bind _output_get (set `self.Health` (- (`self.Health`) Damage)))
  (`BlackboardComponent.SetValueAsObject` (`AIBlueprintHelperLibrary.GetBlackboard` null) "Player" (`GameplayStatics.GetPlayerPawn` 0))
  (set `self.bIsPatrolling` false)
  (if (<= _output_get 0.0)
    (`self.K2_DestroyActor`)))

(event `Patrol`
  (set `CharacterMovementComponent.MaxWalkSpeed` 200.0 (`self.CharacterMovement`))
  (`|AIMoveTo` (`Controller.K2_GetPawn` (`self.GetController`)) (0.0 0.0 0.0) (`|GetArrayItem` (`self.Waypoints`)) 40.0))

(event `Patrol2`
  (bind _returnvalue_x (`KismetMathLibrary.BreakVector` (`self.K2_GetActorLocation`)))
  (bind _returnvalue_x_2 (`KismetMathLibrary.BreakVector` (`self.K2_GetActorLocation` (`GameplayStatics.GetPlayerPawn` 0))))
  (`KismetSystemLibrary.Delay` 1.0)
  (cast `AIController` (`self.GetController`))
  (if (<= (`KismetMathLibrary.Abs` (- _returnvalue_x_2 _returnvalue_x)) (`self.SightDistance`))
    (`KismetSystemLibrary.PrintString` "Catched player!")
    (set `self.bIsPatrolling` false)
    (else
      (`KismetSystemLibrary.PrintString` "Keep patrolling.."))))

(fn `NewFunction`
  (while false
    _))

(fn `UserConstructionScript`)