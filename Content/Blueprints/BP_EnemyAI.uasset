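; Enemy character that patrols waypoints, chases and melees the player, and is destroyed when health runs out.
; Tick walks it between PatrolPoints with movement input and turns its widget toward the camera.
; Sight or damage while patrolling starts timer-looped FollowPlayer, using AIMoveTo, then a montage and sphere-overlap damage.
; ShouldPersue, despite its name, returns true to abandon pursuit once X-axis distance reaches PersueDist, resuming patrol.
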(event `self.PawnSensing.OnSeePawn`
  (params (Pawn :type "Pawn Object Reference"))
  ;[1 1 1] Attack system
  (bind _asbp_third_person_character (cast `/Game/ThirdPerson/Blueprints/BP_ThirdPersonCharacter` Pawn))
  (set `self.SeenPawn` _asbp_third_person_character)
  (set `self.bIsPatrolling` false)
  (set `CharacterMovementComponent.MaxWalkSpeed` 600.0 (`self.CharacterMovement`))
  (`self.FollowPlayer`))

(event `FollowPlayer`
  (bind _seenpawn (`self.SeenPawn`))
  ;[1 1 1] Attack system
  (if (`KismetSystemLibrary.IsValid` _seenpawn)
    (`KismetSystemLibrary.K2_SetTimerDelegate` (delegate `FollowPlayer`) 0.5 true)
    (bind _playergone (`self.ShouldPersue` _seenpawn (`self.PersueDist`)))
    (if _playergone
      (set `self.bIsPatrolling` true)
      (set `self.SeenPawn` null)
      (else
        (`KismetSystemLibrary.PrintString` (`KismetStringLibrary.Conv_BoolToString` _playergone)) ; debug persuefunc
        (`|AIMoveTo` self (0.0 0.0 0.0) _seenpawn 50.0
          (:`OnSuccess`
            (if (`self.bCanAttack`)
              (set `self.bCanAttack` false)
              (bind _returnvalue (`self.PlayAnimMontage` "/Game/Animations/Paired_CounterPunch_PalmStrike_Att_UE5_Montage.Paired_CounterPunch_PalmStrike_Att_UE5_Montage"))
              (bind _outactors (`KismetSystemLibrary.SphereOverlapActors` (`SceneComponent.K2_GetComponentLocation` (`self.Arrow1`)) 100.0 (`self.Object Types`)))
              (for _array_element _outactors
                (if (`self.ActorHasTag` _array_element "Player")
                  (`GameplayStatics.ApplyDamage` _array_element 5.0)))
              (`KismetSystemLibrary.Delay` _returnvalue)
              (set `self.bCanAttack` true))))))))

(event `self.ReceiveTick`
  (params (DeltaSeconds :type "Float (single-precision)"))
  (bind _returnvalue_x (`KismetMathLibrary.BreakVector` (`self.K2_GetActorLocation`)))
  (bind _patrolpoints (`self.PatrolPoints`))
  (bind _waypointtocheck (`self.WaypointToCheck`))
  (bind _waypointtocheck_2 (`self.WaypointToCheck`))
  (bind _output (`|GetArrayItem` _patrolpoints _waypointtocheck))
  (bind _returnvalue_x_2 (`KismetMathLibrary.BreakVector` (`self.K2_GetActorLocation` _output)))
  (bind _returnvalue (`self.GetDistanceTo` _output self))
  (bind _returnvalue_2 (`KismetMathLibrary.FindLookAtRotation` (`KismetMathLibrary.MakeVector` _returnvalue_x) (`KismetMathLibrary.MakeVector` _returnvalue_x_2)))
  (`|ExecutionSequence`
    (:`then_0`
      ;[1 1 1] Handle patrolling
      (if (`self.bIsPatrolling`)
        (set `CharacterMovementComponent.MaxWalkSpeed` 250.0 (`self.CharacterMovement`))
        (if (`KismetArrayLibrary.Array_IsValidIndex` _patrolpoints _waypointtocheck)
          (`self.K2_SetActorRotation` _returnvalue_2)
          (if (> _returnvalue 100.0)
            (`self.AddMovementInput` (`KismetMathLibrary.Conv_RotatorToVector` _returnvalue_2))
            (if (<= _returnvalue 105.0)
              (`KismetSystemLibrary.Delay` 1.5)
              (if (== (- (`KismetArrayLibrary.Array_Length` _patrolpoints) 1) _waypointtocheck_2)
                (set `self.WaypointToCheck` 0)
                (else
                  (set `self.WaypointToCheck` (`KismetMathLibrary.FTrunc` (+ (`KismetMathLibrary.Conv_IntToDouble` _waypointtocheck_2) 1.0))))))))))
    (:`then_1`
      ;[1 1 1] handle camera widget
      (`SceneComponent.K2_SetWorldRotation` (`self.Widget`) (`KismetMathLibrary.FindLookAtRotation` (`SceneComponent.K2_GetComponentLocation` (`self.Widget`)) (`SceneComponent.K2_GetComponentLocation` (`PlayerCameraManager.TransformComponent` (`GameplayStatics.GetPlayerCameraManager` 0)))) false false))))

(event `self.ReceiveAnyDamage`
  (params (Damage :type "Float (single-precision)") (DamageType :type "DamageType Object Reference") (InstigatedBy :type "Controller Object Reference") (DamageCauser :type "Actor Object Reference"))
  ;[1 1 1] Handle damage
  (if (`self.bIsPatrolling`)
    (bind _asbp_third_person_character (cast `/Game/ThirdPerson/Blueprints/BP_ThirdPersonCharacter` (`GameplayStatics.GetPlayerPawn` 0)))
    (set `self.SeenPawn` _asbp_third_person_character)
    (set `self.bIsPatrolling` false)
    (set `CharacterMovementComponent.MaxWalkSpeed` 600.0 (`self.CharacterMovement`))
    (`self.FollowPlayer`))
  (bind _output_get (set `self.Health` (- (`self.Health`) Damage)))
  (`KismetSystemLibrary.PrintString` (`KismetStringLibrary.Conv_DoubleToString` _output_get))
  (if (<= (`self.Health`) 0.0)
    (`self.K2_DestroyActor`)))

(fn `ShouldPersue`
  (params (self2 :type "Actor Object Reference") (persueDist :type "Float (double-precision)"))
  (returns (PlayerGone :type Boolean))
  (bind _returnvalue_x (`KismetMathLibrary.BreakVector` (`self.K2_GetActorLocation` self2)))
  (bind _returnvalue_x_2 (`KismetMathLibrary.BreakVector` (`self.K2_GetActorLocation`)))
  (return (>= (`KismetMathLibrary.Abs` (- _returnvalue_x _returnvalue_x_2)) persueDist)))

(fn `UserConstructionScript`)