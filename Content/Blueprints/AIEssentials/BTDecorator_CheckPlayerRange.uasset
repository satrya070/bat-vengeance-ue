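; Behavior tree decorator that passes while the AI-controlled pawn is within PersueRange of player pawn 0.
; The condition check compares the distance between the two pawns.
; When out of range, it also clears the "Player" blackboard value and sets IsPatrolling on the BaseEnemyOne pawn, so the check has side effects beyond returning its result.
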(fn `PerformConditionCheckAI`
  (params (OwnerController :type "AIController Object Reference") (ControlledPawn :type "Pawn Object Reference"))
  (returns (ReturnValue :type Boolean))
  (bind _returnvalue (< (`Actor.GetDistanceTo` ControlledPawn (`GameplayStatics.GetPlayerPawn` 0)) (`self.PersueRange`)))
  (if (not _returnvalue)
    (`BlackboardComponent.ClearValue` (`AIBlueprintHelperLibrary.GetBlackboard` ControlledPawn) "Player")
    (bind _asbase_enemy_one (cast `/Game/Blueprints/BaseEnemyOne` ControlledPawn))
    (set `/Game/Blueprints/BaseEnemyOne.bIsPatrolling` true _asbase_enemy_one))
  (return _returnvalue))